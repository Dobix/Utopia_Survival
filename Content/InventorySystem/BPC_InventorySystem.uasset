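; Inventory component that holds a slot array, sized to MaxSlotsCount on BeginPlay, and stores items as stacks.
; AddItem uses FindSlotToStore to gather non-full stacks with the same ID, then empty slots if needed.
; It writes the amount into those slots, capping each at the MaxStackSize read from DT_InventoryItems.
; RemoveItem is an empty stub.
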(event EventBeginPlay
  (CallFunction|CreateInventory))

(event EventTick
  (params (DeltaSeconds :type Float%20%28single-precision%29)))

(fn CreateInventory
  (for _index (range 1 (Variables|Default|GetMaxSlotsCount))
    (Utilities|Array|Add :TargetArray (Variables|Default|GetInventory))))

(fn AddItem
  (params (ID :type String) (Amount :type Integer))
  (LocalVariables|SetLocal_AmountLeft Amount)
  (bind _outslots (Searching|FindSlottoStore ID Amount (Searching|FindItems ID)))
  (for _array_element _outslots
    (bind _returnvalue (Utilities|GetDataTableRow "/Game/InventorySystem/DT_InventoryItems.DT_InventoryItems" (Utilities|String|StringToName ID))
      (:then
        (Utilities|Array|SetArrayElem (Variables|Default|GetInventory) (Utilities|Array|FindItem (Variables|Default|GetInventory) _array_element) (Utilities|Struct|MakeS_InventorySlot (Utilities|Struct|MakeDataTableRowHandle "/Game/InventorySystem/DT_InventoryItems.DT_InventoryItems" (Utilities|String|StringToName ID)) (+ (.Amount (Utilities|Struct|BreakS_InventorySlot _array_element)) (Math|Integer|Min(Integer) (- (Utilities|Struct|BreakS_InventoryItem _returnvalue) (.Amount (Utilities|Struct|BreakS_InventorySlot _array_element))) (LocalVariables|GetLocal_AmountLeft))) ID))
        (LocalVariables|SetLocal_AmountLeft (- (LocalVariables|GetLocal_AmountLeft) (Math|Integer|Min(Integer) (- (Utilities|Struct|BreakS_InventoryItem _returnvalue) (.Amount (Utilities|Struct|BreakS_InventorySlot _array_element))) (LocalVariables|GetLocal_AmountLeft))))))))

(fn RemoveItem)

(fn FindItems
  (params (ID :type String))
  (bind _array_element (Utilities|Array|ForEachLoopwithBreak (Variables|Default|GetInventory))
    (:LoopBody
      (if (Utilities|Enum|Equal(Enum) (.ID (Utilities|Struct|BreakS_InventorySlot _array_element)) ID)
        (Utilities|Array|Add (LocalVariables|GetLocal_Slots) _array_element)))
    (:Completed
      (return (LocalVariables|GetLocal_Slots)))))

(fn FindSlottoStore
  (params (ID :type String) (Amount :type Integer) (Slots :type Array%20of%20S%20Inventory%20Slot%20Structures))
  (LocalVariables|SetStorableAmountLeft Amount)
  (bind _array_element (Utilities|Array|ForEachLoopwithBreak Slots :!label _label)
    (:LoopBody
      (bind _returnvalue (Utilities|GetDataTableRow (.DataTable (Utilities|Struct|BreakDataTableRowHandle (.Item (Utilities|Struct|BreakS_InventorySlot _array_element)))) (.RowName (Utilities|Struct|BreakDataTableRowHandle (.Item (Utilities|Struct|BreakS_InventorySlot _array_element)))))
        (:then
          (if (!= (.MaxStackSize (Utilities|Struct|BreakS_InventoryItem _returnvalue)) (.Amount (Utilities|Struct|BreakS_InventorySlot _array_element)))
            (Utilities|Array|Add (LocalVariables|GetLocal_Slots) _array_element)
            (bind _output_get (LocalVariables|SetStorableAmountLeft (Math|Integer|Clamp(Integer) (- (LocalVariables|GetStorableAmountLeft) (Utilities|Operators|Subtract (.MaxStackSize (Utilities|Struct|BreakS_InventoryItem _returnvalue)) (.Amount (Utilities|Struct|BreakS_InventorySlot _array_element)) Amount)) 0 Amount)))
            (if (== _output_get 0)
              (goto _label Break))))))
    (:Completed
      (Utilities|FlowControl|Sequence
        (:then_0
          (if (not (== (LocalVariables|GetStorableAmountLeft) 0))
            (bind _returnvalue_2 (Utilities|GetDataTableRow "/Game/InventorySystem/DT_InventoryItems.DT_InventoryItems" (Utilities|String|StringToName ID))
              (:then
                (bind _array_element_2 (Utilities|Array|ForEachLoopwithBreak (Searching|FindEmptySlots) :!label _label_2)
                  (:LoopBody
                    (LocalVariables|SetStorableAmountLeft (Math|Integer|Clamp(Integer) (- (LocalVariables|GetStorableAmountLeft) (Utilities|Struct|BreakS_InventoryItem _returnvalue_2)) 0 Amount))
                    (Utilities|Array|Add (LocalVariables|GetLocal_Slots) _array_element_2)
                    (if (== (LocalVariables|GetStorableAmountLeft) 0)
                      (goto _label_2 Break))))))))
        (:then_1
          (return (- Amount (LocalVariables|GetStorableAmountLeft)) (LocalVariables|GetLocal_Slots)))))))

(fn FindEmptySlots
  (for _array_element (Variables|Default|GetInventory)
    (if (== (.Amount (Utilities|Struct|BreakS_InventorySlot _array_element)) 0)
      (Utilities|Array|Add (LocalVariables|GetLocal_Slots) _array_element)))
  (return (LocalVariables|GetLocal_Slots)))